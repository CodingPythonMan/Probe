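; Spider turret enemy that wanders to random nearby points until it sees the first-person player, then chases and shoots for the rest of its life.
; PawnSensing sets the active and shooting flags, starting a repeated move-and-face loop toward the player.
; The BeginPlay delay loop switches from wandering to firing projectiles from left and right sockets.
; Player projectile overlaps reduce health with an explosion; death spawns a Time_Fragment.
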(event OnSeePawn(PawnSensing)
  (params (Pawn :type Pawn%20Object%20Reference))
  (bind _self self)
  (bind _asfirst_person_character (Utilities|Casting|CastToFirstPersonCharacter Pawn))
  (Variables|Default|SetAIActive true)
  (Variables|Default|SetisShooting true)
  (AI|AIMoveTo _self "0, 0, 0" _asfirst_person_character 2e+02 false :!label _label
    (:then
      (Transformation|SetActorRotation _self (Math|Rotator|FindLookatRotation (Transformation|GetActorLocation _self) (Transformation|GetActorLocation _asfirst_person_character)))
      (Utilities|FlowControl|Delay 0.5)
      (goto _label))))

(event EventBeginPlay
  ;[1 1 1] 돌아다니기
  (if (Variables|Default|GetAIActive) :!label _label
    ;[1 1 1] 총알 발사
    (if (Variables|Default|GetisShooting) :!label _label_2
      (if (Variables|Default|GetisFirstScan)
        (Utilities|FlowControl|Delay 0.5)
        (Variables|Default|SetisFirstScan false))
      (Game|SpawnActorfromClass "/Game/Enemy/AI_Spider_Turret/Projectile.Projectile_C" (Transformation|GetSocketTransform (Variables|Default|GetSkeletalMesh) "left" "RTS_World") "Undefined" 0 0)
      (Game|SpawnActorfromClass "/Game/Enemy/AI_Spider_Turret/Projectile.Projectile_C" (Transformation|GetSocketTransform (Variables|Default|GetSkeletalMesh) "right" "RTS_World") "Undefined" 0 0)
      (Utilities|FlowControl|Delay 0.4)
      (goto _label_2)
      (else
        (Utilities|FlowControl|Delay 0.0)
        (goto _label_2)))
    (else
      (AI|AIMoveTo self (.RandomLocation (AI|Navigation|GetRandomReachablePointinRadius (Transformation|GetActorLocation) 6e+02 0 0)) 0 5.0 false
        (:OnSuccess
          _)
        (:OnFail
          _))
      (Utilities|FlowControl|Delay 2.0)
      (goto _label))))

(event Collision|EventActorBeginOverlap
  (params (OtherActor :type Actor%20Object%20Reference))
  (Utilities|Casting|CastToFirstPersonProjectile OtherActor)
  (Effects|SpawnEmitteratLocation "/Game/StarterContent/Particles/P_Explosion.P_Explosion" (Transformation|GetWorldLocation (Variables|Collision|GetCapsuleComponent)))
  (bind _output_get (Variables|Default|SetHealth (- (Variables|Default|GetHealth) 0.3)))
  (if (<= _output_get 0.0)
    (Actor|DestroyActor)
    (Game|SpawnActorfromClass "/Game/ITEM/Time_Fragment.Time_Fragment_C" (Transformation|GetActorTransform) "Undefined" 0 0)))

(fn ConstructionScript)