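; Bomb spider enemy that wanders, chases the player when seen, and self-destructs.
; Until AI becomes active, it loops moves to random nearby reachable points; PawnSensing sighting activates it and starts a move toward the player.
; On reaching the player, it sets Armed, then after a short delay spawns an explosion effect and destroys itself.
; Projectile overlaps reduce Health, and death by projectile drops a Time_Fragment.
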(event OnSeePawn(PawnSensing)
  (params (Pawn :type Pawn%20Object%20Reference))
  ;[1 1 1] 플레이어를 발견하였을 때
  (bind _asfirst_person_character (Utilities|Casting|CastToFirstPersonCharacter Pawn))
  (Variables|Default|SetAIActive true)
  (AI|AIMoveTo self "0, 0, 0" _asfirst_person_character 5.0 false
    (:OnSuccess
      (Variables|Default|SetArmed true)
      (Utilities|FlowControl|Delay 3.0)
      (Effects|SpawnEmitteratLocation "/Game/StarterContent/Particles/P_Explosion.P_Explosion" (Transformation|GetActorLocation))
      (Actor|DestroyActor))))

(event EventBeginPlay
  ;[1 1 1] basic AI
  (if (not (Variables|Default|GetAIActive)) :!label _label
    (AI|AIMoveTo self (.RandomLocation (AI|Navigation|GetRandomReachablePointinRadius (Transformation|GetActorLocation) 6e+02 0 0)) 0 5.0 false
      (:OnSuccess
        _)
      (:OnFail
        _))
    (Utilities|FlowControl|Delay 2.0)
    (goto _label)))

(event Collision|EventActorBeginOverlap
  (params (OtherActor :type Actor%20Object%20Reference))
  ;[1 1 1] 총알 맞으면 데미지 & 사망
  (Utilities|Casting|CastToFirstPersonProjectile OtherActor
    (:then
      (Effects|SpawnEmitteratLocation "/Game/StarterContent/Particles/P_Explosion.P_Explosion" (Transformation|GetWorldLocation (Variables|Collision|GetCapsuleComponent)))
      (bind _output_get (Variables|Default|SetHealth (- (Variables|Default|GetHealth) 0.3)))
      (if (<= _output_get 0.0)
        (Actor|DestroyActor)
        (Game|SpawnActorfromClass "/Game/ITEM/Time_Fragment.Time_Fragment_C" (Transformation|GetActorTransform) "Undefined" 0 0)))
    (:CastFailed
      (Development|PrintString "err_spider_bomb"))))

(event EventTick
  (params (DeltaSeconds :type Float%20%28single-precision%29)))

(fn ConstructionScript)