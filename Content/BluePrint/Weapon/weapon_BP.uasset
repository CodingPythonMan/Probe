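; First-person weapon Blueprint that handles automatic fire, ammo and reloading for the player character.
; Pressing fire opens a Gate that loops on a retriggerable delay until release, playing sound and montage and spending ammo per shot.
; A camera line trace sends interface damage with bone name to the hit actor and aims a projectile spawned at the muzzle.
; Releasing fire auto-reloads an empty clip from reserve ammo, with a delay flag blocking fire.
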(event Custom|StartFire
  (bind _characterref (Variables|Default|GetCharacterRef))
  (bind _skeletalmesh (Variables|Default|GetSkeletalMesh))
  (bind _returnvalue (Transformation|GetSocketLocation _skeletalmesh "Muzzle"))
  (bind _firstpersoncamera (Variables|/Game/BluePrint/Character/FirstPersonCharacter.FirstPersonCharacter_C|GetFirstPersonCamera _characterref))
  (bind _returnvalue_2 (Transformation|GetWorldLocation _firstpersoncamera))
  ;[1 1 1] Auto Fire, Hit effect
  (Utilities|FlowControl|Sequence
    (:then_0
      (goto _label Open))
    (:then_1
      (Utilities|FlowControl|Gate true :!label _label
        (:Exit
          (Utilities|FlowControl|Sequence
            (:then_0
              (Utilities|FlowControl|RetriggerableDelay 0.1)
              (goto _label))
            (:then_1
              (if (<= (.CurrentAmmo (Utilities|Struct|BreakWeaponStruct (Variables|Default|GetWeaponInfo))) 0)
                (Development|PrintString "Out of Ammo")
                (else
                  (bind (_outhit _returnvalue_3) (Collision|LineTraceByChannel _returnvalue_2 (+ _returnvalue_2 (* (Math|Vector|GetForwardVector _firstpersoncamera) 1.5e+04)) "TraceTypeQuery1" false 0 "None"))
                  (if _returnvalue_3
                    _
                    (else
                      _))
                  (Audio|PlaySound2D "/Game/Character/FirstPerson/Audio/FirstPersonTemplateWeaponFire02.FirstPersonTemplateWeaponFire02" 1.0 1.0 0.0 0 0)
                  (Animation|PlayAnimMontage (Variables|Default|GetCharacterRef) (Variables|Default|GetPlayFireAnim) 1.0 "None")
                  (bind _structout (Utilities|Struct|SetmembersinWeaponStruct (Variables|Default|GetWeaponInfo) (- (.CurrentAmmo (Utilities|Struct|BreakWeaponStruct (Variables|Default|GetWeaponInfo))) 1)))
                  (CallFunction|OnhitEnemy)
                  (Game|SpawnActorfromClass "/Game/BluePrint/Weapon/FirstPersonProjectile.FirstPersonProjectile_C" (Math|Transform|MakeTransform _returnvalue (Math|Rotator|FindLookatRotation _returnvalue (Math|Vector|SelectVector (.ImpactPoint (Collision|BreakHitResult _outhit)) (.TraceEnd (Collision|BreakHitResult _outhit)) _returnvalue_3))) "Undefined" 0 0))))))))))

(event Custom|StopFire
  (bind _characterref (Variables|Default|GetCharacterRef))
  (bind _skeletalmesh (Variables|Default|GetSkeletalMesh))
  (bind _returnvalue (Transformation|GetSocketLocation _skeletalmesh "Muzzle"))
  (bind _firstpersoncamera (Variables|/Game/BluePrint/Character/FirstPersonCharacter.FirstPersonCharacter_C|GetFirstPersonCamera _characterref))
  (bind _returnvalue_2 (Transformation|GetWorldLocation _firstpersoncamera))
  ;[1 1 1] Auto Fire, Hit effect
  (Utilities|FlowControl|Gate true) ; enters at Close
)

(event Custom|AutoReload
  ;[1 1 1] Auto Reload
  (if (== (.CurrentAmmo (Utilities|Struct|BreakWeaponStruct (Variables|Default|GetWeaponInfo))) 0)
    (if (== (.MaxAmmo (Utilities|Struct|BreakWeaponStruct (Variables|Default|GetWeaponInfo))) 0)
      (Development|PrintString "Find Ammo")
      (else
        (Variables|Default|SetIsReloading true)
        (CallFunction|Reload)))))

(event Custom|Reload
  (bind _weaponinfo (Variables|Default|GetWeaponInfo))
  (bind (_currentammo _objref _clipsize) (Utilities|Struct|BreakWeaponStruct _weaponinfo))
  ;[1 1 1] Reload Check
  (if (== (.MaxAmmo (Utilities|Struct|BreakWeaponStruct (Variables|Default|GetWeaponInfo))) 0)
    (Development|PrintString "Find Ammo")
    (elif (== _currentammo _clipsize)
      (Development|PrintString "Full Ammo")
      (else
        (Variables|Default|SetIsReloading true)
        (CallFunction|WeaponReload)
        (Utilities|FlowControl|Delay 2.0) ; Reloaing Time
        (Variables|Default|SetIsReloading false)))))

(event Custom|Weapon%20Reload
  (bind _weaponinfo (Variables|Default|GetWeaponInfo))
  (bind _weaponinfo_2 (Variables|Default|GetWeaponInfo))
  (bind _weaponinfo_3 (Variables|Default|GetWeaponInfo))
  (bind _weaponinfo_4 (Variables|Default|GetWeaponInfo))
  (bind (_currentammo _clipsize) (Utilities|Struct|BreakWeaponStruct _weaponinfo_3))
  (bind (_currentammo_2 _maxammo) (Utilities|Struct|BreakWeaponStruct _weaponinfo_4))
  (bind _maxammo_2 (Utilities|Struct|BreakWeaponStruct _weaponinfo))
  ;[1 1 1] Actual Weapon Relaod
  (if (> (Utilities|Struct|BreakWeaponStruct (Variables|Default|GetWeaponInfo)) 0)
    (Variables|Default|SetNeededAmmo (- _clipsize _currentammo))
    (if (<= _maxammo_2 (Variables|Default|GetNeededAmmo))
      (Utilities|Struct|SetmembersinWeaponStruct _weaponinfo_2 (+ _currentammo_2 _maxammo))
      (Utilities|Struct|SetmembersinWeaponStruct _weaponinfo_2)
      (else
        (Utilities|Struct|SetmembersinWeaponStruct _weaponinfo_2 (- _maxammo_2 (Variables|Default|GetNeededAmmo)))
        (Utilities|Struct|SetmembersinWeaponStruct _weaponinfo_2 (Utilities|Struct|BreakWeaponStruct (Variables|Default|GetWeaponInfo)))))))

(event Custom|FirePressed
  ;[1 1 1] Do fire from Input
  (Variables|Default|SetCanFire true)
  (if (not (Variables|Default|GetIsReloading))
    (CallFunction|StartFire)))

(event Custom|FireReleased
  ;[1 1 1] Do fire from Input
  (Variables|Default|SetCanFire false)
  (CallFunction|StopFire)
  (CallFunction|AutoReload))

(event Custom|Onhit%20Enemy
  ;[1 1 1] Hit Enemy
  (Class|TakeDamage|ITakeDamage(Message) (.HitActor (Collision|BreakHitResult (stale Custom|StartFire _outhit))) (.HitBoneName (Collision|BreakHitResult (stale Custom|StartFire _outhit))) (Utilities|Struct|BreakWeaponStruct (Variables|Default|GetWeaponInfo))))

(event EventBeginPlay
  ;[1 1 1] get Reference
  (bind _asfirst_person_character (Utilities|Casting|CastToFirstPersonCharacter (Game|GetPlayerCharacter 0)))
  (Variables|Default|SetCharacterRef _asfirst_person_character))

(fn ConstructionScript
  (Variables|Default|SetWeaponInfo (Utilities|Struct|MakeWeaponStruct (.currentammo (Variables|Default|GetWeaponInfo)) (.maxammo (Variables|Default|GetWeaponInfo)) (.damage (Variables|Default|GetWeaponInfo)) (.objref (Variables|Default|GetWeaponInfo)) (.clipsize (Variables|Default|GetWeaponInfo)) (.delay (Variables|Default|GetWeaponInfo)))))